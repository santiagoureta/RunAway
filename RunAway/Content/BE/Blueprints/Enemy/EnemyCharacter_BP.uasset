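; Enemy character Blueprint that chases the player and can be slowed or stunned.
; Ten seconds after BeginPlay it finds the first PlayerCharacter_BP and runs a single AIMoveTo toward it, printing a debug message on success.
; SlowEnemy temporarily lowers max walk speed, while StunEnemy briefly disables movement and sets IsEnemyStunned, both restoring state after timed delays.
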(event `self.ReceiveBeginPlay`
  ;[1 1 1] Begin Play, let the enemy go to the player to kill him
  (`KismetSystemLibrary.Delay` 10.0)
  (bind _outactors (`GameplayStatics.GetAllActorsOfClass` "/Game/BE/Blueprints/Character/PlayerCharacter_BP.PlayerCharacter_BP_C"))
  (bind _output_get (set `self.PlayerCharacterRef` (`|GetArrayItem` _outactors)))
  (`|AIMoveTo` self (0.0 0.0 0.0) _output_get
    (:`OnSuccess`
      (`KismetSystemLibrary.PrintText` "Hello"))))

(event `self.SlowEnemy`
  (bind _charactermovement (`self.CharacterMovement`))
  ;[1 1 1] SLOW ENEMY
  (set `CharacterMovementComponent.MaxWalkSpeed` (`self.EnemySpeedSlowed`) _charactermovement)
  (`KismetSystemLibrary.Delay` 1.5)
  (set `CharacterMovementComponent.MaxWalkSpeed` (`self.EnemyNormalSpeed`) _charactermovement))

(event `self.StunEnemy`
  (bind _charactermovement (`self.CharacterMovement`))
  ;[1 1 1] STUN ENEMY
  (set `self.IsEnemyStunned` true)
  (`CharacterMovementComponent.DisableMovement` _charactermovement)
  (`KismetSystemLibrary.Delay` 1.0)
  (set `self.IsEnemyStunned` false)
  (`CharacterMovementComponent.SetMovementMode` _charactermovement "MOVE_Walking" 0))

(fn `UserConstructionScript`)