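; LightObject_BP is a light actor that reports overlaps to the level illumination system and can flicker or explode.
; While available, it notifies LevelSystemObj when an enemy enters or the player enters or leaves its detection area.
; Timelines drive intensity for flickering, either on its own or as a lead-up to exploding.
; Exploding, delayed or immediate, hides the light, plays a bulb sound and marks it unavailable, disabling those notifications.
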(event `self.ReceiveActorBeginOverlap`
  (params (OtherActor :type "Actor Object Reference"))
  (bind _levelsystemobj (`self.levelSystemObj`))
  ;[1 1 1] Calls to the level ilumination system when the enemy or player entered the light detection sphere
  (if (`self.IsLightAvailable`)
    (bind _asenemy_character_bp (cast `/Game/BE/Blueprints/Enemy/EnemyCharacter_BP` OtherActor)
      (:`then`
        (`LevelSystemIlumination.EnemyOnLight` _levelsystemobj self _asenemy_character_bp))
      (:`CastFailed`
        (cast `/Game/BE/Blueprints/Character/PlayerCharacter_BP` OtherActor)
        (`LevelSystemIlumination.PlayerOnLight` _levelsystemobj self)))
    (else
      (`KismetSystemLibrary.PrintText` "Light is not functional anymore" true true (struct :`G` 0.66 :`B` 1.0 :`A` 1.0) 10.0))))

(event `self.ReceiveActorEndOverlap`
  (params (OtherActor :type "Actor Object Reference"))
  ;[1 1 1] Calls to the level ilumination system when the enemy or player entered the light detection sphere
  (if (`self.IsLightAvailable`)
    (cast `/Game/BE/Blueprints/Character/PlayerCharacter_BP` OtherActor)
    (`LevelSystemIlumination.PlayerOffLight` (`self.levelSystemObj`) self)))

(event `self.FlickeringLight`
  ;[1 1 1] FLICKERING LIGHT
  (bind (_direction _intensity) (`Timeline|Flickering Effect`)
    (:`Update`
      (`LightComponent.SetIntensity` (`self.LightComponent`) (* _intensity 25000.0))
      (set `self.IsLightFlickering` true))))

(event `self.LightToExploteWithDelay`
  (bind _lightcomponent (`self.LightComponent`))
  ;[1 1 1] Explote Light with delay
  (bind (_direction _intensity) (`Timeline|Flicker&Explote`)
    (:`Update`
      (`LightComponent.SetIntensity` _lightcomponent (* _intensity 25000.0))
      (set `self.IsLightFlickering` true))
    (:`Finished`
      (`SceneComponent.SetVisibility` _lightcomponent false false)
      (set `self.IsLightAvailable` false)
      (`GameplayStatics.PlaySoundAtLocation` "/Game/Sounds/BulbExplote_Cue.BulbExplote_Cue" (`SceneComponent.K2_GetComponentLocation` (`self.LightComponent`)) (struct) 1.0 1.0 0.0 null null null))))

(event `self.LightToExplote`
  ;[1 1 1] Light to explote
  (`SceneComponent.SetVisibility` (`self.LightComponent`) false false)
  (set `self.IsLightAvailable` false)
  (`GameplayStatics.PlaySoundAtLocation` "/Game/Sounds/BulbExplote_Cue.BulbExplote_Cue" (`SceneComponent.K2_GetComponentLocation` (`self.LightComponent`)) (struct) 1.0 1.0 0.0 null null null))

(fn `UserConstructionScript`)