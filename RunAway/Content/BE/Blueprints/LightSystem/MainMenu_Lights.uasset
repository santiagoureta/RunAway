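; Main menu light actor that can flicker a spotlight with accompanying sound when IsFlickering is set.
; On BeginPlay, a timeline drives the spotlight intensity through a scaled curve and keeps the sound playing until it finishes.
; Each update also toggles the skeletal mesh, showing it only when the curve drops below zero.
; Non-flickering lights stop the sound and hide the mesh.
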(event `self.ReceiveBeginPlay`
  (bind _sound (`self.Sound`))
  (bind _skeletalmesh (`self.SkeletalMesh`))
  (if (`self.IsFlickering`)
    (bind (_direction _intensity) (`Timeline|FlickeringLineTime`)
      (:`Update`
        (if (>= _intensity 0.0)
          (`SceneComponent.SetVisibility` _skeletalmesh false false)
          (else
            (`SceneComponent.SetVisibility` _skeletalmesh true false)))
        (`LightComponent.SetIntensity` (`self.SpotLight`) (* _intensity 25000.0))
        (if (not (`AudioComponent.IsPlaying` _sound))
          (`AudioComponent.Play` _sound 0.0)))
      (:`Finished`
        (`AudioComponent.Stop` (`self.Sound`))))
    (else
      (`AudioComponent.Stop` (`self.Sound`))
      (`SceneComponent.SetVisibility` (`self.SkeletalMesh`) false false))))

(fn `UserConstructionScript`)